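; Hostile spawner actor that spawns AI_Hostile_WFC enemies at its Sphere component while spawning is switched on.
; On BeginPlay it gets the player controller through a message call and binds to its start and stop spawning dispatchers.
; Start opens a Gate that re-enters itself after a fixed delay for repeated spawns, and stop closes it.
; The MaxAmountAI-capped loop and another spawn loop are disconnected, so no cap applies.
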(event Custom|Dispatcher_StartSpawning_Event
  (bind _sphere (Variables|Default|GetSphere))
  (bind _returnvalue (Transformation|GetWorldTransform _sphere))
  (Utilities|FlowControl|Sequence
    (:then_0
      (goto _label Open))
    (:then_1
      (Utilities|FlowControl|Gate true :!label _label
        (:Exit
          (Game|SpawnActorfromClass "/Game/Assets/Hostile/WFC/AI_Hostile_WFC.AI_Hostile_WFC_C" (Math|Transform|MakeTransform (.location _returnvalue) (.rotation _returnvalue) "1,1,1") "Undefined" 0 0)
          (Utilities|FlowControl|Delay 3.0)
          (goto _label))))))

(event Custom|Dispatcher_StopSpawning_Event
  (bind _sphere (Variables|Default|GetSphere))
  (bind _returnvalue (Transformation|GetWorldTransform _sphere))
  (Utilities|FlowControl|Gate true) ; enters at Close
)

(event EventBeginPlay
  (bind _bp_mcontroller (Class|BPIPlayerController|ControllerReference(Message) (Game|GetPlayerController 0)))
  (Variables|Default|SetBP%20MController _bp_mcontroller)
  (EventDispatchers|AssignDispatcherStartSpawning (Variables|Default|GetBP%20MController) (delegate Custom|Dispatcher_StartSpawning_Event))
  (EventDispatchers|AssignDispatcherStopSpawning (Variables|Default|GetBP%20MController) (delegate Custom|Dispatcher_StopSpawning_Event)))

(fn ConstructionScript)
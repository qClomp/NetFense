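; BP_HostileSpawner is a spawner actor that produces AI_Hostile_WFC hostiles at its Sphere component's location and rotation.
; On BeginPlay it spawns one, waits on a fixed delay, increments LoopCounter, and loops back until the count reaches MaxAmountAI.
; The limit is checked after each spawn, so at least one hostile always spawns.
; An unconnected copy of the loop without a limit remains in the graph and never runs.
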(event EventBeginPlay
  (bind _sphere (Variables|Default|GetSphere))
  (bind _returnvalue (Transformation|GetWorldTransform _sphere))
  (Game|SpawnActorfromClass "/Game/Assets/Hostile/WFC/AI_Hostile_WFC.AI_Hostile_WFC_C" (Math|Transform|MakeTransform (.location _returnvalue) (.rotation _returnvalue) "1,1,1") "Undefined" 0 0 :!label _label)
  (Utilities|FlowControl|Delay 3.0)
  (bind _output_get (Variables|Default|Setloop_counter (+ (Variables|Default|Getloop_counter) 1)))
  (if (< _output_get (Variables|Default|Getmax_amount_AI))
    (goto _label)))

(fn ConstructionScript)
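; Player controller for a building game that turns input into camera pawn movement, spring arm zoom, build menu toggling, demolition and save/load.
; Clicks, Alt, demolish and save broadcast through dispatchers, while loading calls ACLoadGame directly and ACDemolish is initialised on BeginPlay.
; Interface messages fetch the pawn, toggle HUD UI and expose the controller and build component.
; Old screen-edge scrolling and save/load test code remain unwired.
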(event EventBeginPlay
  (bind _mplayer (Class|BPIMPlayer|MPlayerGetReference(Message) (Game|Player|GetPlayerPawn 0)))
  (Variables|Default|SetMPlayer _mplayer)
  (Default|InitDemolish (Variables|Default|GetAC_Demolish) self))

(event EventTick
  (params (DeltaSeconds :type Float%20%28single-precision%29)))

(event Input|ActionEvents|InputActionInput_MouseRightClick
  (params (Key :type Key%20Structure :default "None"))
  (:Pressed
    (Default|CallDispatcherMouseRightClick)))

(event Input|ActionEvents|InputActionInput_MouseLeftClick
  (params (Key :type Key%20Structure :default "None"))
  (:Pressed
    (Default|CallDispatcherMouseLeftClick)))

(event Input|ActionEvents|InputActionInput_Alt
  (params (Key :type Key%20Structure :default "None"))
  (:Pressed
    (bind _isa (Utilities|FlowControl|FlipFlop)
      (:A
        _)
      (:B
        _))
    (Default|CallDispatcherKeyALT (not _isa))))

(event Input|ActionEvents|InputActionInput_SaveGame
  (params (Key :type Key%20Structure :default "None"))
  (:Pressed
    (Default|CallDispatcherSaveGame)))

(event Input|ActionEvents|InputActionInput_Demolish
  (params (Key :type Key%20Structure :default "None"))
  (:Pressed
    (Default|CallDispatcherDemolish)))

(event Input|ActionEvents|InputActionInput_LoadGame
  (params (Key :type Key%20Structure :default "None"))
  (:Pressed
    (Default|ELoadSavedGame (Variables|Default|GetAC_LoadGame))))

(event Input|AxisEvents|InputAxisInput_MouseRightClick
  (params (AxisValue :type Float%20%28single-precision%29))
  ;[1 1 1] Movement
  ;;[1 0 0] DEACTIVATED
)

(event Input|AxisEvents|InputAxisInput_MoveUpDown
  (params (AxisValue :type Float%20%28single-precision%29))
  ;[1 1 1] Movement
  (Pawn|Input|AddMovementInput (Variables|Default|GetMPlayer) (Math|Vector|GetForwardVector (Variables|/Game/Player/BP_MPlayer.BP_MPlayer_C|GetDirectionArrow (Variables|Default|GetMPlayer))) AxisValue false))

(event Input|AxisEvents|InputAxisInput_MoveRightLeft
  (params (AxisValue :type Float%20%28single-precision%29))
  ;[1 1 1] Movement
  (Pawn|Input|AddMovementInput (Variables|Default|GetMPlayer) (Math|Vector|GetRightVector (Variables|/Game/Player/BP_MPlayer.BP_MPlayer_C|GetDirectionArrow (Variables|Default|GetMPlayer))) AxisValue false))

(event Input|AxisEvents|InputAxisMoveForward
  (params (AxisValue :type Float%20%28single-precision%29))
  ;[1 1 1] Movement
  (Pawn|Input|AddMovementInput (Variables|Default|GetMPlayer) (Math|Vector|GetForwardVector (Variables|/Game/Player/BP_MPlayer.BP_MPlayer_C|GetDirectionArrow (Variables|Default|GetMPlayer))) AxisValue false))

(event Input|AxisEvents|InputAxisMoveRight
  (params (AxisValue :type Float%20%28single-precision%29))
  ;[1 1 1] Movement
  (Pawn|Input|AddMovementInput (Variables|Default|GetMPlayer) (Math|Vector|GetRightVector (Variables|/Game/Player/BP_MPlayer.BP_MPlayer_C|GetDirectionArrow (Variables|Default|GetMPlayer))) AxisValue false))

(event Input|AxisEvents|InputAxisInput_MouseWheel
  (params (AxisValue :type Float%20%28single-precision%29))
  (bind _mplayer (Variables|Default|GetMPlayer))
  (bind _springarm (Variables|/Game/Player/BP_MPlayer.BP_MPlayer_C|GetSpringArm _mplayer))
  (if (!= AxisValue 0.0)
    (Variables|/Script/Engine.SpringArmComponent|SetTargetArmLength _springarm (+ (Variables|/Script/Engine.SpringArmComponent|GetTargetArmLength _springarm) (* AxisValue -1e+02)))))

(event Input|KeyboardEvents|1
  (params (Key :type Key%20Structure :default "None"))
  (:Pressed
    (Class|BPIHUD|ToggleVisibilityUIBuildModule(Message) (HUD|GetHUD))))

(fn ConstructionScript)

(fn ControllerModuleBuildReference
  (return (Variables|Default|GetBPActorComponent_BuildModule)))

(fn ControllerReference
  (return self))
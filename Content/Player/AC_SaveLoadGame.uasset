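; Player component that saves and restores placed server, turret and TCP modules and the cables between them through a Save_MySaveGame slot.
; Saving gathers save structs from each actor via messages, appends them to arrays and writes the slot asynchronously after each group.
; Loading spawns every saved module before passing each its data by matching array index, then spawns the cables and loads theirs.
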(event Custom|E_SaveGame
  ;[1 1 1] Save
  (Development|PrintString "Save Game Started")
  (Utilities|FlowControl|Sequence
    (:then_0
      (bind _outactors (Actor|GetAllActorsOfClass "/Game/Assets/Modules/Network_Modules/ServerV1/Module_ServerV1.Module_ServerV1_C"))
      (CallFunction|ESaveModules _outactors)
      (bind _outactors_2 (Actor|GetAllActorsOfClass "/Game/Assets/Modules/Defense_Modules/TurretV1/Module_TurretV1.Module_TurretV1_C"))
      (CallFunction|ESaveModules _outactors_2)
      (bind _outactors_3 (Actor|GetAllActorsOfClass "/Game/Assets/Modules/Connection_Modules/TCPV1/Module_TCPV1.Module_TCPV1_C"))
      (CallFunction|ESaveModules _outactors_3))
    (:then_1
      ;[1 1 1] Cable
      (bind _outactors_4 (Actor|GetAllActorsOfClass "/Game/Assets/Modules/Connection_Modules/CableV1/Module_CableV1.Module_CableV1_C"))
      (for _array_element _outactors_4
        (bind _save_cable (Default|CableSaveData _array_element))
        (Utilities|Array|Add (Variables|SaveData|GetSave%20Cables) _save_cable))
      (bind _savegame_object (Variables|!!SaveGameObject|GetSaveGame%20Object)
        (:then
          (Variables|/Game/Levels/ProjectSamples/Save_MySaveGame.Save_MySaveGame_C|SetSave%20Cables _savegame_object (Variables|SaveData|GetSave%20Cables))
          (|AsyncSaveGametoSlot _savegame_object (Variables|SaveID|GetSave_SlotName) (Variables|Default|GetUser%20Index)))
        (:else)))))

(event Custom|E_Save%20Modules
  (params (Actors%20Array :type Array%20of%20Object%20Object%20References))
  (bind _save_modules (Variables|SaveData|GetSave%20Modules))
  (for _array_element Actors%20Array
    (bind (_succes _save_module) (Class|BPIModules|ModuleSaveData(Message) _array_element))
    (if _succes
      (Utilities|Array|Add _save_modules _save_module)
      (Development|PrintString (Utilities|String|ToString(Integer) (Utilities|Array|Length _save_modules)))))
  (bind _savegame_object (Variables|!!SaveGameObject|GetSaveGame%20Object)
    (:then
      (Variables|/Game/Levels/ProjectSamples/Save_MySaveGame.Save_MySaveGame_C|SetSaved%20Modules _savegame_object (Variables|SaveData|GetSave%20Modules))
      (|AsyncSaveGametoSlot _savegame_object (Variables|SaveID|GetSave_SlotName) (Variables|Default|GetUser%20Index)))
    (:else)))

(event Custom|E_LoadGame
  ;[1 1 1] Load
  (bind _returnvalue (SaveGame|DoesSaveGameExist (Variables|SaveID|GetSave_SlotName) (Variables|Default|GetUser%20Index)))
  (if _returnvalue
    (bind _savegame (|AsyncLoadGamefromSlot (Variables|SaveID|GetSave_SlotName) (Variables|Default|GetUser%20Index))
      (:Completed
        (bind _assave_my_save_game (Utilities|Casting|CastToSave_MySaveGame _savegame)
          (:then
            (Variables|!!SaveGameObject|SetLoaded%20Save%20Game _assave_my_save_game)
            (Utilities|FlowControl|Sequence
              (:then_0
                (for _array_element (Variables|/Game/Levels/ProjectSamples/Save_MySaveGame.Save_MySaveGame_C|GetSaved%20Modules (Variables|!!SaveGameObject|GetLoaded%20Save%20Game))
                  (bind _returnvalue_2 (Game|SpawnActorfromClass (.ActorClass (Utilities|Struct|BreakStructure_Save_Module _array_element)) (.WorldTransform (Utilities|Struct|BreakStructure_Save_Module _array_element)) "Undefined" 0 0))
                  (Utilities|Array|Add (Variables|Default|GetSpawnedActors) _returnvalue_2)
                  (Development|PrintString (Utilities|GetDisplayName (.TurretConnectedProtocol (Utilities|Struct|BreakStructure_Save_Module _array_element))))
                  (Development|PrintString (Utilities|String|Append (Utilities|GetDisplayName (.ConnectedTargetIOStream (Utilities|Struct|BreakStructure_Save_IOStream (.IOStreamSaveData (Utilities|Struct|BreakStructure_Save_Module _array_element))))) (Utilities|GetDisplayName (.ConnectedModule (Utilities|Struct|BreakStructure_Save_IOStream (.IOStreamSaveData (Utilities|Struct|BreakStructure_Save_Module _array_element))))) (Utilities|GetDisplayName (.CableReference (Utilities|Struct|BreakStructure_Save_IOStream (.IOStreamSaveData (Utilities|Struct|BreakStructure_Save_Module _array_element))))))))
                (for (_array_element_2 _array_index) (Variables|/Game/Levels/ProjectSamples/Save_MySaveGame.Save_MySaveGame_C|GetSaved%20Modules (Variables|!!SaveGameObject|GetLoaded%20Save%20Game))
                  (Class|BPIModules|ModuleLoadData(Message) (Utilities|Array|Get(acopy) (Variables|Default|GetSpawnedActors) _array_index) _array_element_2)))
              (:then_1
                (for _array_element_3 (Variables|/Game/Levels/ProjectSamples/Save_MySaveGame.Save_MySaveGame_C|GetSave%20Cables (Variables|!!SaveGameObject|GetLoaded%20Save%20Game))
                  (bind _returnvalue_3 (Game|SpawnActorfromClass (.ActorClass (Utilities|Struct|BreakStructure_Save_Cable _array_element_3)) (Math|Transform|MakeTransform "0, 0, 0" "0, 0, 0" "1,1,1") "Undefined" 0 0))
                  (Class|BPICableModule|CableLoadData(Message) _returnvalue_3 _array_element_3)))))
          (:CastFailed
            (Development|PrintString "MySaveGame | Cast Failed")))))))

(event EventBeginPlay
  ;[1 1 1] Begin Play
  (bind _returnvalue (SaveGame|CreateSaveGameObject "/Game/Levels/ProjectSamples/Save_MySaveGame.Save_MySaveGame_C"))
  (Variables|!!SaveGameObject|SetSaveGame%20Object _returnvalue))
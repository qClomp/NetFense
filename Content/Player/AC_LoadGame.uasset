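; Player-side component that saves and restores the world's Module_ServerV1 actors through a Save_MySaveGame slot.
; BeginPlay creates a fresh save object; E_SaveGame appends each module's data to SaveModules, never cleared here, then writes it asynchronously.
; E_LoadGame reads the slot asynchronously, spawns each saved class at its stored transform and passes it the record via LoadModuleMessage, without removing existing modules.
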(event Custom|E_LoadGame
  (bind _savegame (|AsyncLoadGamefromSlot (Variables|Default|GetSave_SlotName))
    (:Completed
      (bind _assave_my_save_game (Utilities|Casting|CastToSave_MySaveGame _savegame))
      (for _array_element (Variables|/Game/Levels/ProjectSamples/Save_MySaveGame.Save_MySaveGame_C|GetSaved%20Modules _assave_my_save_game)
        (bind _returnvalue (Game|SpawnActorfromClass (.ActorClass (Utilities|Struct|BreakStructure_SaveModule _array_element)) (.WorldTransform (Utilities|Struct|BreakStructure_SaveModule _array_element)) "Undefined" 0 0))
        (Class|BPISaveLoadGame|LoadModule(Message) _returnvalue _array_element)
        (Development|PrintString "Loaded")))))

(event Custom|E_SaveGame
  (Development|PrintString "Save Game Started")
  (bind _outactors (Actor|GetAllActorsOfClass "/Game/Assets/Modules/Network_Modules/ServerV1/Module_ServerV1.Module_ServerV1_C"))
  (for _array_element _outactors
    (bind _savemodule (Default|GetModuleSaveData _array_element))
    (Utilities|Array|Add (Variables|Default|GetSave_Modules) _savemodule))
  (bind _savegame_object (Variables|Default|GetSaveGame%20Object)
    (:then
      (Variables|/Game/Levels/ProjectSamples/Save_MySaveGame.Save_MySaveGame_C|SetSaved%20Modules _savegame_object (Variables|Default|GetSave_Modules))
      (|AsyncSaveGametoSlot _savegame_object (Variables|Default|GetSave_SlotName)))
    (:else)))

(event EventBeginPlay
  ;[1 1 1] Begin Play
  (bind _returnvalue (SaveGame|CreateSaveGameObject "/Game/Levels/ProjectSamples/Save_MySaveGame.Save_MySaveGame_C"))
  (Variables|Default|SetSaveGame%20Object _returnvalue))
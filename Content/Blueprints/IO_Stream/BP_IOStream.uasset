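; BP_IOStream is a cable port that links its owning module to one other IOStream and relays network bandwidth between them.
; Connecting stores a single target, greets it with itself and notifies the module, while a scene point marks the cable location.
; Send and use calls for download and upload route by source: module calls go to the target stream, target calls go to the module, both returning the result.
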(event Custom|E_ProtocolConnected
  ;[0 0 0] Do we really need this ?
)

(event EventIOStreamInitModule
  (params (Connected_Module :type Actor%20Object%20Reference) (IOStream%20Type :type enum_IOStreamType%20Enum :default "NewEnumerator0"))
  (Variables|Connections|SetConnected%20Module Connected_Module)
  (Variables|Default|SetIOStream%20Type IOStream%20Type))

(event EventIOStreamCableConnected
  ;[0 0 0] Do we really need this ?
  (Class|BPIModules|ModuleCableConnected(Message) (Variables|Connections|GetConnected%20Module)))

(fn ConstructionScript
  (Transformation|SetRelativeLocation (Variables|Default|GetCableLocation) (Variables|Default|GetCableLoc) false false))

(fn IOStreamCanConnect?
  (return (not (Utilities|IsValid (Variables|Connections|GetConnected%20Target%20IOStream)))))

(fn IOStreamConnecttoTarget
  (params (Client :type Actor%20Object%20Reference))
  (Utilities|IsValid (Variables|Connections|GetConnected%20Target%20IOStream)
    (:Is%20Valid
      (return false))
    (:Is%20Not%20Valid
      (bind _output_get (Variables|Connections|SetConnected%20Target%20IOStream Client))
      ;[1 1 1] Say Hello To Target IOStream
      (Class|BPIIOStream|IOStreamConnecttoTarget(Message) _output_get self)
      (Utilities|FlowControl|Sequence
        (:then_0
          (Class|BPIModules|ModuleCableConnected(Message) (Variables|Connections|GetConnected%20Module)))
        (:then_1
          (return (Utilities|IsValid (Variables|Connections|GetConnected%20Target%20IOStream))))))))

(fn IOStreamGetCableLocation
  (return (Transformation|GetWorldLocation (Variables|Default|GetCableLocation))))

(fn IOStreamSendNetworkConnection
  (params (Source :type Actor%20Object%20Reference) (Download :type Float%20%28single-precision%29) (Upload :type Float%20%28single-precision%29))
  (if (== (Variables|Connections|GetConnected%20Target%20IOStream) Source)
    (bind (_used _takendownload _takenupload) (Class|BPIModules|ModuleSendNetwork(Message) (Variables|Connections|GetConnected%20Module) Download Upload))
    (return _used _takendownload _takenupload)
    (elif (== (Variables|Connections|GetConnected%20Module) Source)
      (bind (_used_ _useddownload _usedupload) (Class|BPIIOStream|IOStreamSendNetworkConnection(Message) (Variables|Connections|GetConnected%20Target%20IOStream) self Download Upload))
      (return _used_ _useddownload _usedupload))))

(fn IOStreamUseNetwork
  (params (Source :type Actor%20Object%20Reference) (UsedDownload :type Float%20%28single-precision%29) (UsedUpload :type Float%20%28single-precision%29))
  (if (== Source (Variables|Connections|GetConnected%20Module))
    (bind _succes (Class|BPIIOStream|IOStreamUseNetwork(Message) (Variables|Connections|GetConnected%20Target%20IOStream) self UsedDownload UsedUpload))
    (return _succes)
    (elif (== Source (Variables|Connections|GetConnected%20Target%20IOStream))
      (bind _succes_2 (Class|BPIModules|ModuleUseNetwork(Message) (Variables|Connections|GetConnected%20Module) UsedDownload UsedUpload))
      (return _succes_2)
      (else
        (return false)))))
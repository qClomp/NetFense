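; Actor component for module building: spawns a module actor from a given structure and moves it with the mouse cursor.
; BuildModule spawns it below the world origin, then a looping timer at the tick delta snaps it to the cursor's Visibility trace hit.
; A left-click dispatcher from the player controller, obtained by message, pauses that timer through a gate.
; The module's collision overlaps are bound but only print debug text.
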(event Custom|init_Dispatchers
  (EventDispatchers|AssignDispatcherMouseLeftClick (Variables|Default|GetPlayerController) (delegate Custom|Dispatcher_MouseLeftClick_Event_0)))

(event Custom|E_MoveCurrentBuild
  (bind _current_buildactor (Variables|Default|GetCurrent_BuildActor)
    (:then
      (Transformation|SetActorLocation _current_buildactor (.location (.HitResult (Game|Player|GetHitResultUnderCursorbyChannel (Variables|Default|GetPlayerController) "TraceTypeQuery1" true))) false false))
    (:else)))

(event Custom|E_CurrentModuleCollision
  (bind _modulecollision (Class|BPIModules|ModuleGetCollision(Message) (Variables|Default|GetCurrent_BuildActor)))
  (Utilities|FlowControl|Sequence
    (:then_0
      (Collision|AssignOnComponentBeginOverlap _modulecollision (delegate Custom|OnComponentBeginOverlap_Event_Module)))
    (:then_1
      (Collision|AssignOnComponentEndOverlap _modulecollision (delegate Custom|OnComponentEndOverlap_Event_Module)))))

(event Custom|Dispatcher_MouseLeftClick_Event_0
  (Utilities|FlowControl|Gate false
    (:Exit
      (Utilities|Time|PauseTimerbyHandle (Variables|Default|GetTimer_MoveCurrentBuild)))))

(event Custom|OnComponentBeginOverlap_Event_Module
  (params (OverlappedComponent :type Primitive%20Component%20Object%20Reference) (OtherActor :type Actor%20Object%20Reference) (OtherComp :type Primitive%20Component%20Object%20Reference) (OtherBodyIndex :type Integer) (bFromSweep :type Boolean) (SweepResult :type Hit%20Result%20Structure%20%28by%20ref%29))
  (Development|PrintString "BeginOverlap!"))

(event Custom|OnComponentEndOverlap_Event_Module
  (params (OverlappedComponent :type Primitive%20Component%20Object%20Reference) (OtherActor :type Actor%20Object%20Reference) (OtherComp :type Primitive%20Component%20Object%20Reference) (OtherBodyIndex :type Integer))
  (Development|PrintString "EndOverlap!"))

(event EventBeginPlay
  (bind _bp_mcontroller (Class|BPIMController|ControllerReference(Message) (Game|GetPlayerController 0)))
  (Variables|Default|SetPlayerController _bp_mcontroller)
  (CallFunction|InitDispatchers))

(event EventTick
  (params (DeltaSeconds :type Float%20%28single-precision%29))
  (Variables|Default|SetDelta%20Seconds DeltaSeconds))

(event EventBuildModule
  (params (ModuleStructure :type Structure%20Module%20Specifications%20Structure))
  (bind _moduleactorclass (Utilities|Struct|BreakStructure_ModuleSpecifications ModuleStructure))
  (if (Utilities|IsValidClass _moduleactorclass)
    (bind _returnvalue (Game|SpawnActorfromClass _moduleactorclass (Math|Transform|MakeTransform "0, 0,-5000.000000" "0, 0, 0" "1,1,1") "Undefined" 0 0))
    (Variables|Default|SetCurrent_BuildActor _returnvalue)
    (bind _returnvalue_2 (Utilities|Time|SetTimerbyEvent (delegate Custom|E_MoveCurrentBuild) (Variables|Default|GetDelta%20Seconds) true))
    (Variables|Default|SetTimer_MoveCurrentBuild _returnvalue_2)
    (CallFunction|ECurrentModuleCollision)))
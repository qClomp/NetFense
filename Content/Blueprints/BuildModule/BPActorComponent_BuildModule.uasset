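; Actor component that handles player placement of build modules, protocols and IO cables via mouse clicks.
; BuildModule spawns the actor by build type, and looping timers move it to the cursor hit point.
; Overlap events swap green/red materials to show validity: modules need clear space, protocols a compatible module, cables two IOStream endpoints.
; Left click confirms and restores materials, while right click cancels, with interface messages handling connections.
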(event Custom|init_Dispatchers
  (Utilities|FlowControl|Sequence
    (:then_0
      ;[1 1 1] Mouse Right Click
      (EventDispatchers|AssignDispatcherMouseRightClick (Variables|Player|GetPlayerController) (delegate Custom|Dispatcher_MouseRightClick_Event)))
    (:then_1
      ;[1 1 1] Dispatchers
      ;;[1 1 1] Mouse Left Click
      (EventDispatchers|AssignDispatcherMouseLeftClick (Variables|Player|GetPlayerController) (delegate Custom|Dispatcher_MouseLeftClick_Event_0)))))

(event Custom|E_MoveCable
  ;[1 1 1] Build Cable
  (bind _current_buildactor (Variables|CurrentActor|GetCurrent_BuildActor)
    (:then
      (Transformation|SetActorLocation _current_buildactor (Utilities|MHitResult) false false))
    (:else)))

(event Custom|Build_Default
  (bind _module_collision (Variables|CurrentActor|GetModule%20Collision))
  (bind _module_collision_2 (Variables|CurrentActor|GetModule%20Collision))
  (bind _structure_buildactor (Variables|CurrentActor|GetStructure_BuildActor))
  ;[1 1 1] Build Default
  (if (Utilities|IsValidClass (.moduleactorclass _structure_buildactor))
    (bind _returnvalue (Game|SpawnActorfromClass (.moduleactorclass _structure_buildactor) (Math|Transform|MakeTransform "0, 0,-5000.000000" "0, 0, 0" "1,1,1") "Undefined" 0 0))
    (bind _output_get (Variables|CurrentActor|SetCurrent_BuildActor _returnvalue))
    (CallFunction|EGetCurrentModuleVariables _output_get)
    (bind _returnvalue_2 (Utilities|Time|SetTimerbyEvent (delegate Custom|E_MoveCurrentBuild) (Variables|SelfVariables|GetDelta%20Seconds) true))
    (Variables|Timer|SetTimer_MoveCurrentBuild _returnvalue_2)
    ;;[1 1 1] Dividing Protocol and Default
    (switch Utilities|FlowControl|Switch|SwitchonENUM_BuildType (.buildtype (Variables|CurrentActor|GetStructure_BuildActor))
      (:NewEnumerator0
        ;[1 1 1] Default Collision
        (Utilities|FlowControl|Sequence
          (:then_0
            (Variables|Buildable_Booleans|SetDefault_Buildable true)
            (Rendering|Material|SetMaterial (Variables|CurrentActor|GetModule%20Mesh) 0 "/Game/Blueprints/BuildModule/M_CollisionGreen.M_CollisionGreen"))
          (:then_1
            (Collision|AssignOnComponentBeginOverlap _module_collision_2 (delegate Custom|OnComponentBeginOverlap_Event_Module)))
          (:then_2
            (Collision|AssignOnComponentEndOverlap _module_collision_2 (delegate Custom|OnComponentEndOverlap_Event_Module)))))
      (:NewEnumerator2
        ;[1 1 1] Protocol Collision
        (Utilities|FlowControl|Sequence
          (:then_0
            (Rendering|Material|SetMaterial (Variables|CurrentActor|GetModule%20Mesh) 0 "/Game/Blueprints/BuildModule/M_CollisionRed.M_CollisionRed"))
          (:then_1
            (Collision|AssignOnComponentBeginOverlap _module_collision (delegate Custom|OnComponentBeginOverlap_Event_0)))
          (:then_2
            (Collision|BindEventtoOnComponentEndOverlap _module_collision (delegate Custom|OnComponentEndOverlap_Event_0))))))))

(event Custom|OnComponentBeginOverlap_Event_Cable
  (params (OverlappedComponent :type Primitive%20Component%20Object%20Reference) (OtherActor :type Actor%20Object%20Reference) (OtherComp :type Primitive%20Component%20Object%20Reference) (OtherBodyIndex :type Integer) (bFromSweep :type Boolean) (SweepResult :type Hit%20Result%20Structure%20%28by%20ref%29))
  ;[1 1 1] Cable Collision
  (if (Actor|ActorHasTag OtherActor "IOStream")
    (bind _succes (Class|BPIIOStream|IOStreamCanConnect?(Message) OtherActor))
    (if _succes
      (Variables|Cable|SetCable_Touching%20IOStream OtherActor)
      (Variables|Cable|SetCableTouchingConnectable true)
      (Rendering|Material|SetMaterial (Variables|Cable|GetCableMesh) 0 "/Game/Blueprints/BuildModule/M_CollisionGreen.M_CollisionGreen"))))

(event Custom|OnComponentEndOverlap_Event_Cable
  (params (OverlappedComponent :type Primitive%20Component%20Object%20Reference) (OtherActor :type Actor%20Object%20Reference) (OtherComp :type Primitive%20Component%20Object%20Reference) (OtherBodyIndex :type Integer))
  ;[1 1 1] Cable Collision
  (Variables|Cable|SetCableTouchingConnectable false)
  (Variables|Buildable_Booleans|SetCable_Buildable false)
  (Rendering|Material|SetMaterial (Variables|Cable|GetCableMesh) 0 "/Game/Blueprints/BuildModule/M_CollisionRed.M_CollisionRed"))

(event Custom|E_DragCableEnd
  ;[1 1 1] Cable
  (Class|BPICableModule|CableSetEnd(Message) (Variables|CurrentActor|GetCurrent_BuildActor) (Utilities|MHitResult)))

(event Custom|Dispatcher_MouseRightClick_Event
  ;[1 1 1] Mouse Right Click
  (switch Utilities|FlowControl|Switch|SwitchonENUM_BuildType (.buildtype (Variables|CurrentActor|GetStructure_BuildActor))
    (:NewEnumerator0
      (Utilities|Time|PauseTimerbyHandle (Variables|Timer|GetTimer_MoveCurrentBuild) :!label _label))
    (:NewEnumerator1
      (Utilities|Time|PauseTimerbyHandle (Variables|Timer|GetTimer_MoveCable))
      (Utilities|Time|PauseTimerbyHandle (Variables|Timer|GetTimer_DragCableEnd)))
    (:NewEnumerator2
      (goto _label)))
  (bind _current_buildactor (Variables|CurrentActor|GetCurrent_BuildActor)
    (:then
      (Actor|DestroyActor _current_buildactor)
      (Utilities|MCleanCableVariables))
    (:else)))

(event Custom|E_MoveCurrentBuild
  ;[1 1 1] Build Default
  (bind _current_buildactor (Variables|CurrentActor|GetCurrent_BuildActor)
    (:then
      (Transformation|SetActorLocation _current_buildactor (Utilities|MHitResult) false false))
    (:else)))

(event Custom|OnComponentBeginOverlap_Event_Module
  (params (OverlappedComponent :type Primitive%20Component%20Object%20Reference) (OtherActor :type Actor%20Object%20Reference) (OtherComp :type Primitive%20Component%20Object%20Reference) (OtherBodyIndex :type Integer) (bFromSweep :type Boolean) (SweepResult :type Hit%20Result%20Structure%20%28by%20ref%29))
  ;[1 1 1] Default Collision
  (Variables|CurrentActor|GetModule%20Collision
    (:then
      (Variables|Buildable_Booleans|SetDefault_Buildable false)
      (Rendering|Material|SetMaterial (Variables|CurrentActor|GetModule%20Mesh) 0 "/Game/Blueprints/BuildModule/M_CollisionRed.M_CollisionRed"))
    (:else)))

(event Custom|OnComponentEndOverlap_Event_Module
  (params (OverlappedComponent :type Primitive%20Component%20Object%20Reference) (OtherActor :type Actor%20Object%20Reference) (OtherComp :type Primitive%20Component%20Object%20Reference) (OtherBodyIndex :type Integer))
  ;[1 1 1] Default Collision
  (Variables|CurrentActor|GetModule%20Collision
    (:then
      (Variables|Buildable_Booleans|SetDefault_Buildable true)
      (Rendering|Material|SetMaterial (Variables|CurrentActor|GetModule%20Mesh) 0 "/Game/Blueprints/BuildModule/M_CollisionGreen.M_CollisionGreen"))
    (:else)))

(event Custom|OnComponentBeginOverlap_Event_0
  (params (OverlappedComponent :type Primitive%20Component%20Object%20Reference) (OtherActor :type Actor%20Object%20Reference) (OtherComp :type Primitive%20Component%20Object%20Reference) (OtherBodyIndex :type Integer) (bFromSweep :type Boolean) (SweepResult :type Hit%20Result%20Structure%20%28by%20ref%29))
  (bind _returnvalue (Components|GetOwner OtherComp))
  ;[1 1 1] Protocol Collision
  (if (Components|ComponentHasTag OtherComp "Protocol_IN")
    (bind _boolean (Class|BPIModules|ModuleHasProtocol?(Message) _returnvalue))
    (if _boolean
      (Variables|Default|SetProtocol_Overlapping_Module _returnvalue)
      ;[1 1 1] State For Buildable & Color
      (Variables|CurrentActor|GetModule%20Collision
        (:then
          (Variables|Default|SetProtocol_Buildable true)
          (Rendering|Material|SetMaterial (Variables|CurrentActor|GetModule%20Mesh) 0 "/Game/Blueprints/BuildModule/M_CollisionGreen.M_CollisionGreen"))
        (:else)))))

(event Custom|OnComponentEndOverlap_Event_0
  (params (OverlappedComponent :type Primitive%20Component%20Object%20Reference) (OtherActor :type Actor%20Object%20Reference) (OtherComp :type Primitive%20Component%20Object%20Reference) (OtherBodyIndex :type Integer))
  ;[1 1 1] Protocol Collision
  (Variables|CurrentActor|GetModule%20Collision
    (:then
      (Variables|Default|SetProtocol_Buildable false)
      (Rendering|Material|SetMaterial (Variables|CurrentActor|GetModule%20Mesh) 0 "/Game/Blueprints/BuildModule/M_CollisionRed.M_CollisionRed"))
    (:else)))

(event Custom|Dispatcher_MouseLeftClick_Event_0
  ;[1 1 1] Dispatchers
  (switch Utilities|FlowControl|Switch|SwitchonENUM_BuildType (.buildtype (Variables|CurrentActor|GetStructure_BuildActor))
    (:NewEnumerator0
      ;;[1 1 1] Default Build
      (if (Variables|Buildable_Booleans|GetDefault_Buildable)
        (Utilities|Time|PauseTimerbyHandle (Variables|Timer|GetTimer_MoveCurrentBuild) :!label _label)
        (Variables|CurrentActor|GetCurrent_BuildActor
          (:then
            (for (_array_element _array_index) (Variables|CurrentActor|GetModuleMaterials)
              (Rendering|Material|SetMaterial (Variables|CurrentActor|GetModule%20Mesh) _array_index _array_element)
              ;;[1 1 1] Garbage Collector
              (Utilities|MCleanBuildVariables)))
          (:else))))
    (:NewEnumerator1
      ;[1 1 1] Cable
      (if (Variables|Cable|GetCableTouchingConnectable)
        (if (Utilities|Time|IsTimerActivebyHandle (Variables|Timer|GetTimer_DragCableEnd))
          (bind _cable_touching_iostream (Variables|Cable|GetCable_Touching%20IOStream)
            (:then
              (bind _succes (Class|BPIIOStream|IOStreamConnecttoTarget(Message) _cable_touching_iostream (Variables|Cable|GetCable_SourceActor)))
              (if _succes
                (Variables|Cable|SetCableTouchingConnectable false)
                (Utilities|Time|PauseTimerbyHandle (Variables|Timer|GetTimer_DragCableEnd))
                ;;[1 1 1] Sets Cable End Location (Connected Actor)
                ;;;[0 0 0] CHANGE (Cable Loc)
                (bind _location (Class|BPIIOStream|IOStreamGetCableLocation(Message) (Variables|Cable|GetCable_Touching%20IOStream)))
                (Class|BPICableModule|CableSetEnd(Message) (Variables|CurrentActor|GetCurrent_BuildActor) _location)
                ;[1 1 1] Material
                (for (_array_element_2 _array_index_2) (Variables|Cable|GetCable_Materials)
                  (Rendering|Material|SetMaterial (Variables|Cable|GetCableMesh) _array_index_2 _array_element_2)
                  ;[1 1 1] Garbage Collector
                  (Utilities|MCleanCableVariables))))
            (:else))
          (else
            (Utilities|Time|PauseTimerbyHandle (Variables|Timer|GetTimer_MoveCable))
            ;;[1 1 1] Gets Touched Current IOStream for further usage
            (bind _output_get (Variables|Cable|SetCable_SourceActor (Variables|Cable|GetCable_Touching%20IOStream)))
            ;;[0 0 0] CHANGE (Cable Loc)
            (bind _location_2 (Class|BPIIOStream|IOStreamGetCableLocation(Message) _output_get))
            (Class|BPICableModule|CableSetStart(Message) (Variables|CurrentActor|GetCurrent_BuildActor) _location_2)
            (bind _returnvalue (Utilities|Time|SetTimerbyEvent (delegate Custom|E_DragCableEnd) (Variables|SelfVariables|GetDelta%20Seconds) true))
            (Variables|Timer|SetTimer_DragCableEnd _returnvalue)))))
    (:NewEnumerator2
      ;;[1 1 1] Protocol Connects To Module
      (if (Variables|Default|GetProtocol_Buildable)
        (bind _succes_2 (Class|BPIModules|ConnecttoProtocolModule(Message) (Variables|Default|GetProtocol_Overlapping_Module) (Variables|CurrentActor|GetCurrent_BuildActor)))
        (if _succes_2
          (bind _succes_3 (Class|BPIModules|ConnecttoModuleProtocol(Message) (Variables|CurrentActor|GetCurrent_BuildActor) (Variables|Default|GetProtocol_Overlapping_Module)))
          (if _succes_3
            (goto _label)))))))

(event Custom|E_GetCurrentModuleVariables
  (params (BuildActor :type Actor%20Object%20Reference))
  ;[1 1 1] Set Current Build Variables
  (bind (_modulecollision _moduleskeletalmesh) (Class|BPIModules|ModuleGetCollisionandMesh(Message) BuildActor))
  (Variables|CurrentActor|SetModule%20Collision _modulecollision)
  (bind _output_get (Variables|CurrentActor|SetModule%20Mesh _moduleskeletalmesh))
  (Variables|CurrentActor|SetModuleMaterials (Rendering|Material|GetMaterials _output_get)))

(event Custom|Build_Spline/Cable
  (bind _structure_buildactor (Variables|CurrentActor|GetStructure_BuildActor))
  ;[1 1 1] Build Cable
  (if (Utilities|IsValidClass (.moduleactorclass _structure_buildactor))
    (bind _returnvalue (Game|SpawnActorfromClass (.moduleactorclass _structure_buildactor) (Math|Transform|MakeTransform "0, 0,-5000.000000" "0, 0, 0" "1,1,1") "Undefined" 0 0))
    (bind _output_get (Variables|CurrentActor|SetCurrent_BuildActor _returnvalue))
    (CallFunction|EGetCableVariables _output_get)
    (bind _returnvalue_2 (Utilities|Time|SetTimerbyEvent (delegate Custom|E_MoveCable) (Variables|SelfVariables|GetDelta%20Seconds) true))
    (Variables|Timer|SetTimer_MoveCable _returnvalue_2)
    ;[1 1 1] Cable Collision
    (Utilities|FlowControl|Sequence
      (:then_0
        (Rendering|Material|SetMaterial (Variables|Cable|GetCableMesh) 0 "/Game/Blueprints/BuildModule/M_CollisionRed.M_CollisionRed"))
      (:then_1
        (Collision|AssignOnComponentBeginOverlap (Variables|Cable|GetCableCollision) (delegate Custom|OnComponentBeginOverlap_Event_Cable)))
      (:then_2
        (Collision|AssignOnComponentEndOverlap (Variables|Cable|GetCableCollision) (delegate Custom|OnComponentEndOverlap_Event_Cable))))))

(event Custom|E_GetCableVariables
  (params (CableActor :type Actor%20Object%20Reference))
  ;[1 1 1] Get Cable Variables
  (bind (_splinecollision _splinemesh) (Class|BPICableModule|GetCableVariables(Message) CableActor))
  (Variables|Cable|SetCableCollision _splinecollision)
  (bind _output_get (Variables|Cable|SetCableMesh _splinemesh))
  (Variables|Cable|SetCable_Materials (Rendering|Material|GetMaterials _output_get)))

(event EventBeginPlay
  ;[1 1 1] Begin play & Event tick
  (bind _bp_mcontroller (Class|BPIPlayerController|ControllerReference(Message) (Game|GetPlayerController 0)))
  (Variables|Player|SetPlayerController _bp_mcontroller)
  (CallFunction|InitDispatchers))

(event EventTick
  (params (DeltaSeconds :type Float%20%28single-precision%29))
  ;[1 1 1] Begin play & Event tick
  (Variables|SelfVariables|SetDelta%20Seconds DeltaSeconds))

(event EventBuildModule
  (params (ModuleStructure :type Structure%20Module%20Specifications%20Structure))
  ;[1 1 1] BuildModule_MainCall
  (bind _output_get (Variables|CurrentActor|SetStructure_BuildActor ModuleStructure))
  (switch Utilities|FlowControl|Switch|SwitchonENUM_BuildType (.buildtype _output_get)
    (:NewEnumerator0
      (CallFunction|BuildDefault :!label _label))
    (:NewEnumerator1
      (CallFunction|BuildSpline/Cable))
    (:NewEnumerator2
      (goto _label))))

(fn FCleanCollisionEvents
  (bind _module_collision (Variables|CurrentActor|GetModule%20Collision)
    (:then
      (EventDispatchers|UnbindallEventsfromOnComponentBeginOverlap _module_collision)
      (EventDispatchers|UnbindallEventsfromOnComponentEndOverlap _module_collision))
    (:else
      _))
  (bind _cablecollision (Variables|Cable|GetCableCollision)
    (:then
      (EventDispatchers|UnbindallEventsfromOnComponentBeginOverlap _cablecollision)
      (EventDispatchers|UnbindallEventsfromOnComponentEndOverlap _cablecollision))
    (:else)))
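; Demolish component that, so far, only prints debug names as groundwork for a demolish mode; nothing is destroyed.
; init_Demolish stores a controller reference and binds to its Demolish dispatcher.
; Each dispatch flip-flops between starting a roughly 60 Hz looping timer and pausing it, with the timer printing the M_HitResult macro's display name.
; The macro's under-cursor Visibility trace appears unconnected.
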(event Custom|init_Demolish
  (params (Controller%20Reference :type BP%20M%20Controller%20Object%20Reference))
  (bind _output_get (Variables|Default|SetController%20Reference Controller%20Reference))
  (EventDispatchers|AssignDispatcherDemolish _output_get (delegate Custom|Dispatcher_Demolish_Event)))

(event Custom|Dispatcher_Demolish_Event
  (Utilities|FlowControl|FlipFlop
    (:A
      (bind _returnvalue (Utilities|Time|SetTimerbyEvent (delegate Custom|E_HitResult) 0.016667 true))
      (Variables|Default|Settimer_HitResult _returnvalue))
    (:B
      (Utilities|Time|PauseTimerbyHandle (Variables|Default|Gettimer_HitResult)))))

(event Custom|E_HitResult
  (Development|PrintString (Utilities|GetDisplayName (Utilities|MHitResult))))

(event EventBeginPlay)

(event EventTick
  (params (DeltaSeconds :type Float%20%28single-precision%29)))